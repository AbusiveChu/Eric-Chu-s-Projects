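; Tetris stored-piece display that shows the held tetromino as colored cubes on a small grid.
; BeginPlay defines the seven shapes as cell indices, builds a 4×2 grid of hidden cube components, and fills a matching position lookup.
; ChangeStoredPiece converts the piece type to a numeric ID for SwapSP, which clears the grid and resolves the shape's cells.
; MakeBlocks reveals those cubes, records their type and applies the piece's color material.
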(event Custom|SwapSP
  (params (PieceTypeToStore :type Integer))
  (Utilities|Array|Clear (Variables|Default|GetCurrentStoredPositions))
  (CallFunction|ClearGrid)
  (bind _output_get (Variables|Default|SetStoredPieceType PieceTypeToStore))
  (for _array_element (Utilities|Struct|BreakTetrominoShapes (Utilities|Array|Get(acopy) (Variables|Default|GetShapes) (- _output_get 2)))
    (Utilities|Array|Add (Variables|Default|GetCurrentStoredPositions) (Utilities|Array|Get(acopy) (Variables|Default|GetSpawnPositions) _array_element)))
  (CallFunction|MakeBlocks (Variables|Default|GetCurrentStoredPositions) (Variables|Default|GetStoredPieceType)))

(event Custom|ChangeStoredPiece
  (params (InPieceType :type PieceShape%20Enum :default "NewEnumerator0"))
  (switch Utilities|FlowControl|Switch|SwitchonPieceShape InPieceType
    (:NewEnumerator0
      (Variables|Default|SetStoredPieceType 2))
    (:NewEnumerator1
      (Variables|Default|SetStoredPieceType 3))
    (:NewEnumerator2
      (Variables|Default|SetStoredPieceType 4))
    (:NewEnumerator3
      (Variables|Default|SetStoredPieceType 5))
    (:NewEnumerator4
      (Variables|Default|SetStoredPieceType 6))
    (:NewEnumerator5
      (Variables|Default|SetStoredPieceType 7))
    (:NewEnumerator6
      (Variables|Default|SetStoredPieceType 8)))
  (CallFunction|SwapSP (Variables|Default|GetStoredPieceType)))

(event EventBeginPlay
  (bind _rowcounter (Variables|Default|GetRowCounter))
  (bind _grid (Variables|Default|GetGrid))
  (bind _shapes (Variables|Default|GetShapes))
  (bind _boxspacing (Variables|Default|GetBoxSpacing))
  (bind _output (Utilities|Array|Get(acopy) _grid _rowcounter))
  (bind (_blocktypes _meshes) (Utilities|Struct|BreakRow _output))
  (Utilities|FlowControl|Sequence
    (:then_0
      (Utilities|FlowControl|Sequence
        (:then_0
          ;[1 1 1] I Block
          (Utilities|Array|Add _shapes (Utilities|Struct|MakeTetrominoShapes (Utilities|Array|MakeArray 1 3 5 7))))
        (:then_1
          ;[1 1 1] Z Block
          (Utilities|Array|Add _shapes (Utilities|Struct|MakeTetrominoShapes (Utilities|Array|MakeArray 2 4 5 7))))
        (:then_2
          ;[1 1 1] S Block
          (Utilities|Array|Add _shapes (Utilities|Struct|MakeTetrominoShapes (Utilities|Array|MakeArray 3 5 4 6))))
        (:then_3
          ;[1 1 1] T Block
          (Utilities|Array|Add _shapes (Utilities|Struct|MakeTetrominoShapes (Utilities|Array|MakeArray 3 5 4 7))))
        (:then_4
          ;[1 1 1] L Block
          (Utilities|Array|Add _shapes (Utilities|Struct|MakeTetrominoShapes (Utilities|Array|MakeArray 2 5 7 3))))
        (:then_5
          ;[1 1 1] J Block
          (Utilities|Array|Add _shapes (Utilities|Struct|MakeTetrominoShapes (Utilities|Array|MakeArray 3 5 7 6))))
        (:then_6
          ;[1 1 1] O Block
          (Utilities|Array|Add _shapes (Utilities|Struct|MakeTetrominoShapes (Utilities|Array|MakeArray 2 3 4 5))))))
    (:then_1
      (for _index (range 0 3)
        (for _index_2 (range 0 1)
          (bind _returnvalue (AddComponent|AddStaticMeshComponent false (Math|Transform|MakeTransform (Math|Vector|MakeVector (* _index _boxspacing) 0.0 (* _index_2 _boxspacing)))))
          (Components|StaticMesh|SetStaticMesh _returnvalue "/Game/StarterContent/Shapes/Shape_Cube.Shape_Cube")
          (Rendering|SetVisibility _returnvalue false false)
          (if (== (Variables|Default|GetGridCounter) 0)
            (Utilities|Array|Add (Variables|Default|GetGrid) (Utilities|Struct|MakeRow (Utilities|Array|MakeArray 0) (Utilities|Array|MakeArray _returnvalue)))
            (else
              (Utilities|Array|Add _blocktypes 0)
              (Utilities|Array|Add _meshes _returnvalue)))
          (bind _result (Math|Integer|IncrementInt (Variables|Default|GetGridCounter))
            (:%20%20
              (if (== _result 2)
                (Variables|Default|SetGridCounter 0)
                (Math|Integer|IncrementInt (Variables|Default|GetRowCounter))))))))
    (:then_2
      (for _index_3 (range 0 3)
        (for _index_4 (range 0 1)
          (Utilities|Array|Add (Variables|Default|GetSpawnPositions) (Utilities|Struct|MakeGridPosition _index_4 _index_3)))))))

(fn ConstructionScript)

(fn MakeBlocks
  (params (BlocksToMake :type Array%20of%20Grid%20Position%20Structures) (BlockType :type Integer))
  (for _array_element BlocksToMake
    (Rendering|SetVisibility (Utilities|Array|Get(acopy) (.Meshes (Utilities|Struct|BreakRow (Utilities|Array|Get(acopy) (Variables|Default|GetGrid) (.y (Utilities|Struct|BreakGridPosition _array_element))))) (.x (Utilities|Struct|BreakGridPosition _array_element))) true false)
    (Utilities|Array|SetArrayElem (.BlockTypes (Utilities|Struct|BreakRow (Utilities|Array|Get(acopy) (Variables|Default|GetGrid) (.y (Utilities|Struct|BreakGridPosition _array_element))))) (.x (Utilities|Struct|BreakGridPosition _array_element)) BlockType)
    (switch int BlockType
      (:2
        (Rendering|Material|SetMaterial (Utilities|Array|Get(acopy) (.Meshes (Utilities|Struct|BreakRow (Utilities|Array|Get(acopy) (Variables|Default|GetGrid) (.y (Utilities|Struct|BreakGridPosition _array_element))))) (.x (Utilities|Struct|BreakGridPosition _array_element))) 0 "/Game/Tetris/TetrisMaterials/Teal.Teal"))
      (:3
        (Rendering|Material|SetMaterial (Utilities|Array|Get(acopy) (.Meshes (Utilities|Struct|BreakRow (Utilities|Array|Get(acopy) (Variables|Default|GetGrid) (.y (Utilities|Struct|BreakGridPosition _array_element))))) (.x (Utilities|Struct|BreakGridPosition _array_element))) 0 "/Game/Tetris/TetrisMaterials/Red.Red"))
      (:4
        (Rendering|Material|SetMaterial (Utilities|Array|Get(acopy) (.Meshes (Utilities|Struct|BreakRow (Utilities|Array|Get(acopy) (Variables|Default|GetGrid) (.y (Utilities|Struct|BreakGridPosition _array_element))))) (.x (Utilities|Struct|BreakGridPosition _array_element))) 0 "/Game/Tetris/TetrisMaterials/Green.Green"))
      (:5
        (Rendering|Material|SetMaterial (Utilities|Array|Get(acopy) (.Meshes (Utilities|Struct|BreakRow (Utilities|Array|Get(acopy) (Variables|Default|GetGrid) (.y (Utilities|Struct|BreakGridPosition _array_element))))) (.x (Utilities|Struct|BreakGridPosition _array_element))) 0 "/Game/Tetris/TetrisMaterials/Purple.Purple"))
      (:6
        (Rendering|Material|SetMaterial (Utilities|Array|Get(acopy) (.Meshes (Utilities|Struct|BreakRow (Utilities|Array|Get(acopy) (Variables|Default|GetGrid) (.y (Utilities|Struct|BreakGridPosition _array_element))))) (.x (Utilities|Struct|BreakGridPosition _array_element))) 0 "/Game/Tetris/TetrisMaterials/Orange.Orange"))
      (:7
        (Rendering|Material|SetMaterial (Utilities|Array|Get(acopy) (.Meshes (Utilities|Struct|BreakRow (Utilities|Array|Get(acopy) (Variables|Default|GetGrid) (.y (Utilities|Struct|BreakGridPosition _array_element))))) (.x (Utilities|Struct|BreakGridPosition _array_element))) 0 "/Game/Tetris/TetrisMaterials/Blue.Blue"))
      (:8
        (Rendering|Material|SetMaterial (Utilities|Array|Get(acopy) (.Meshes (Utilities|Struct|BreakRow (Utilities|Array|Get(acopy) (Variables|Default|GetGrid) (.y (Utilities|Struct|BreakGridPosition _array_element))))) (.x (Utilities|Struct|BreakGridPosition _array_element))) 0 "/Game/Tetris/TetrisMaterials/Yellow.Yellow")))))

(fn ClearGrid
  (for _index (range 0 3)
    (for _index_2 (range 0 1)
      (Rendering|SetVisibility (Utilities|Array|Get(acopy) (.Meshes (Utilities|Struct|BreakRow (Utilities|Array|Get(acopy) (Variables|Default|GetGrid) _index))) _index_2) false false)
      (Utilities|Array|SetArrayElem (.BlockTypes (Utilities|Struct|BreakRow (Utilities|Array|Get(acopy) (Variables|Default|GetGrid) _index))) _index_2 0))))
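; Forklift actor that raises and lowers its tongs and can kill the player, ending the game.
; The construction script stores the tongs' starting position as lowered and a point above it as raised.
; Each tick interpolates the tongs toward one of them based on IsForkUp, which is set outside these graphs.
; While IsForkUp is false, a MainCharacter overlapping the forklift triggers the game over menu, UI-only input and pause.
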(event EventTick
  (params (DeltaSeconds :type Float%20%28single-precision%29))
  (Variables|Default|SetCurrentVec (Transformation|GetWorldLocation (Variables|Default|GetForkliftTongs)))
  (if (Variables|Default|GetIsForkUp?)
    (Transformation|SetWorldLocation (Variables|Default|GetForkliftTongs) (Math|Interpolation|VInterpTo (Transformation|GetWorldLocation (Variables|Default|GetForkliftTongs)) (Variables|Default|GetRaisedVec) DeltaSeconds 1.0) false)
    (else
      (Transformation|SetWorldLocation (Variables|Default|GetForkliftTongs) (Math|Interpolation|VInterpTo (Transformation|GetWorldLocation (Variables|Default|GetForkliftTongs)) (Variables|Default|GetLoweredVec) DeltaSeconds 1.0) false)
      (if (== (Utilities|Array|Length (Collision|GetOverlappingActors "/Game/MainCharacter.MainCharacter_C" :!class /Script/Engine.PrimitiveComponent)) 1)
        (bind _returnvalue (UserInterface|CreateWidget "/Game/Menus/GameOverMenu.GameOverMenu_C"))
        (UserInterface|Viewport|AddtoViewport _returnvalue 0)
        (Input|SetInputModeUIOnly (Game|GetPlayerController 0) _returnvalue false)
        (Game|SetGamePaused true)))))

(fn ConstructionScript
  (bind _output_get (Variables|Default|SetLoweredVec (Transformation|GetWorldLocation (Variables|Default|GetForkliftTongs))))
  (Variables|Default|SetRaisedVec (Math|Vector|MakeVector (.X (Math|Vector|BreakVector _output_get)) (.Y (Math|Vector|BreakVector _output_get)) (+ (.Z (Math|Vector|BreakVector _output_get)) 1.5e+02))))
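; MainHUD is a HUD Blueprint that draws temporary on-screen messages for locked, boarded or blocked doors, plus the player's key count.
; DrawHUD checks boolean flags in priority order, draws the first active message and clears its flag after a short Delay.
; The key count branch reads NumberOfKeys from MainCharacter and uses a DoOnce to toggle its KeyCounterIcon around the Delay before resetting.
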(event EventDrawHUD
  (params (SizeX :type Integer) (SizeY :type Integer))
  (bind _returnvalue (Math|Conversions|ToFloat(Integer) SizeY))
  (bind _returnvalue_2 (Math|Conversions|ToFloat(Integer) SizeX))
  (bind _returnvalue_3 (Game|GetPlayerController 0))
  (bind _returnvalue_4 (/ _returnvalue 2.0))
  (bind _returnvalue_5 (/ _returnvalue_2 2.0))
  (bind _returnvalue_6 (Game|GetPlayerCharacter _returnvalue_3))
  (if (Variables|Default|GetDoorLocked)
    (HUD|DrawText "Door is Locked, Key Required" "(R=1.000000,G=1.000000,B=1.000000,A=1.000000)" _returnvalue_5 _returnvalue_4 0 3.0 false)
    (Utilities|FlowControl|Delay 2.0)
    (Variables|Default|SetDoorLocked false)
    (elif (Variables|Default|GetScriptDoorisLocked)
      (HUD|DrawText "Door is Locked,  Black Key is Required" "(R=0.995000,G=0.995000,B=0.995000,A=1.000000)" 0.0 _returnvalue_4 0 3.0 false)
      (Utilities|FlowControl|Delay 2.0)
      (Variables|Default|SetScriptDoorisLocked false)
      (elif (Variables|Default|GetMetalDoorLocked)
        (HUD|DrawText "Metal Door is Locked,  2 Keys Required" "(R=0,G=0,B=0,A=1)" _returnvalue_5 _returnvalue_4 0 3.0 false)
        (Utilities|FlowControl|Delay 2.0)
        (Variables|Default|SetMetalDoorLocked false)
        (elif (Variables|Default|GetDoorBoarded)
          (HUD|DrawText "Door is Boarded, Find something to break it!" "(R=0,G=0,B=0,A=1)" 0.0 0.0 0 3.0 false)
          (Utilities|FlowControl|Delay 2.0)
          (Variables|Default|SetDoorBoarded false)
          (elif (Variables|Default|GetDoorisBlocked)
            (HUD|DrawText "This Door is Blocked" "(R=0,G=0,B=0,A=1)" 0.0 0.0 0 3.0 false)
            (Utilities|FlowControl|Delay 2.0)
            (Variables|Default|SetDoorisBlocked false)
            (elif (Variables|Default|GetKeyCount)
              (bind _asmain_character (Utilities|Casting|CastToMainCharacter _returnvalue_6))
              (HUD|DrawText (Utilities|String|Append (Utilities|String|ToString(Integer) (Variables|/Game/MainCharacter.MainCharacter_C|GetNumberOfKeys _asmain_character)) " x") "(R=1.000000,G=1.000000,B=1.000000,A=1.000000)" (/ _returnvalue_5 3.0) (* _returnvalue_4 1.5) 0 3.0 false)
              (Utilities|FlowControl|DoOnce false :!label _label
                (:Completed
                  (bind _asmain_character_2 (Utilities|Casting|CastToMainCharacter _returnvalue_6))
                  (Rendering|ToggleVisibility (Variables|/Game/MainCharacter.MainCharacter_C|GetKeyCounterIcon _asmain_character_2) false)
                  (Utilities|FlowControl|Delay 2.0)
                  (Rendering|ToggleVisibility (Variables|/Game/MainCharacter.MainCharacter_C|GetKeyCounterIcon _asmain_character_2) false)
                  (Variables|Default|SetKeyCount false)
                  (goto _label Reset))))))))))

(fn ConstructionScript)
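; Spot light Blueprint that flickers with a brief spark sound while its IsOn flag is true.
; Tick runs a chain of fixed, uneven Delays that toggle visibility, relying on latent delays to pace the repeating pattern.
; Each pass ends with a short Activate/Deactivate burst and a quiet, attenuated spark sound at the actor's location.
; BeginPlay starts with that burst component deactivated.
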(event EventTick
  (params (DeltaSeconds :type Float%20%28single-precision%29))
  (if (Variables|Default|GetIsOn)
    (Utilities|FlowControl|Delay 0.05)
    (Rendering|ToggleVisibility false)
    (Utilities|FlowControl|Delay 0.05)
    (Rendering|ToggleVisibility false)
    (Utilities|FlowControl|Delay 0.2)
    (Rendering|ToggleVisibility false)
    (Utilities|FlowControl|Delay 0.5)
    (Rendering|ToggleVisibility false)
    (Utilities|FlowControl|Delay 0.2)
    (Rendering|ToggleVisibility false)
    (Utilities|FlowControl|Delay 1.5)
    (Rendering|ToggleVisibility false)
    (Components|Activation|Activate false)
    (Utilities|FlowControl|Delay 0.1)
    (Components|Activation|Deactivate)
    (Audio|PlaySoundatLocation "/Game/Assets/Audio/reflect_spark_02.reflect_spark_02" (Transformation|GetActorLocation) 0.01 1.0 0.0 "/Game/Assets/Audio/water_drips_att.water_drips_att")))

(event EventBeginPlay
  (Components|Activation|Deactivate))

(fn ConstructionScript)
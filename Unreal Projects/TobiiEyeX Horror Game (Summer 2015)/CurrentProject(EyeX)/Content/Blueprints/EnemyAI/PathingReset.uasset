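; Behavior tree task that clears the PathSet blackboard key and moves the enemy AI's pawn to the NextPathingLocation vector.
; It caches the EnemyAIController on first execution and runs AIMoveTo on its controlled pawn, finishing successfully on arrival.
; A failed move fails the task and prints the movement result unless it matches BlockedCheck.
; An AbortCheck failure branch is present but never runs.
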(event EventReceiveExecute
  (params (OwnerActor :type Actor%20Object%20Reference))
  (if (!= (Variables|Default|GetAI%20CON%20Ref) 0)
    _
    (else
      (bind _asenemy_aicontroller (Utilities|Casting|CastToEnemyAIController OwnerActor))
      (Variables|Default|SetAI%20CON%20Ref _asenemy_aicontroller)))
  (Class|BTFunctionLibrary|ClearBlackboardValue (Variables|Default|GetPathSet))
  (bind _movementresult (AI|AIMoveTo (Pawn|GetControlledPawn (Variables|Default|GetAI%20CON%20Ref)) (Class|BTFunctionLibrary|GetBlackboardValueasVector (Variables|Default|GetNextPathingLocation)) 0 5.0 false)
    (:OnSuccess
      (AI|BehaviorTree|FinishExecute true))
    (:OnFail
      (if (== _movementresult (Variables|Default|GetBlocked%20Check))
        (AI|BehaviorTree|FinishExecute false)
        (else
          (Development|PrintString (Utilities|String|EnumtoString _movementresult))
          (AI|BehaviorTree|FinishExecute false))))))
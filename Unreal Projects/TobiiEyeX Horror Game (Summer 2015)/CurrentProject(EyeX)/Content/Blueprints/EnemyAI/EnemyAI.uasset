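; EnemyAI is an enemy pawn Blueprint that drives audio playback from the state of its EnemyAIController.
; Each Tick casts the controller, starts playback if its State is 1 and nothing is playing, and stops playback for any other state.
; The Audio component's finished event restarts playback without checking the state.
; A GettingUp animation branch is present but never runs.
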(event OnAudioFinished(Audio)
  (Audio|Components|Audio|Play 0.0))

(event EventTick
  (params (DeltaSeconds :type Float%20%28single-precision%29))
  (bind _asenemy_aicontroller (Utilities|Casting|CastToEnemyAIController (Pawn|GetController)))
  (if (== (Variables|/Game/Blueprints/EnemyAI/EnemyAIController.EnemyAIController_C|GetState _asenemy_aicontroller) 1)
    (bind _returnvalue (Audio|Components|Audio|IsPlaying))
    (if (not _returnvalue)
      (Audio|Components|Audio|Play 0.0))
    (else
      (Audio|Components|Audio|Stop))))

(fn ConstructionScript)
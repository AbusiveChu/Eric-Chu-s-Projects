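; AggroStart is an enemy AI behavior tree node that keeps the blackboard aimed at the player during aggro.
; Each tick it uses the EnemyAIController, cast from the owner and cached on first use, to write the player pawn and location as follow targets.
; It halves MoveSpeed while the controller reports both HasGaze and Detection.
; It also gathers all EnemyAI actors and the pawn's location, but uses neither.
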(event EventTick
  (params (OwnerActor :type Actor%20Object%20Reference) (DeltaSeconds :type Float%20%28single-precision%29))
  (bind _returnvalue (Game|Player|GetPlayerPawn 0))
  ;[1 1 1] Is AI_CON_Ref set?
  (if (!= (Variables|Default|GetAI_CON_Ref) 0)
    _
    (else
      (bind _asenemy_aicontroller (Utilities|Casting|CastToEnemyAIController OwnerActor))
      (Variables|Default|SetAI_CON_Ref _asenemy_aicontroller)))
  (Actor|GetAllActorsOfClass "/Game/Blueprints/EnemyAI/EnemyAI.EnemyAI_C")
  (Variables|Default|SetMyLocation (Transformation|GetActorLocation (Pawn|GetControlledPawn (Variables|Default|GetAI_CON_Ref))))
  (if (and (Variables|/Game/Blueprints/EnemyAI/EnemyAIController.EnemyAIController_C|GetHasGaze _asenemy_aicontroller) (Variables|/Game/Blueprints/EnemyAI/EnemyAIController.EnemyAIController_C|GetDetection? _asenemy_aicontroller))
    (Class|BTFunctionLibrary|SetBlackboardValueasFloat (Variables|Default|GetMoveSpeed) 1e+02)
    (else
      (Class|BTFunctionLibrary|SetBlackboardValueasFloat (Variables|Default|GetMoveSpeed) 2e+02)))
  (Class|BTFunctionLibrary|SetBlackboardValueasObject (Variables|Default|GetTargetToFollow) _returnvalue)
  (AI|BehaviorTree|SetBlackboardValueasVector (Variables|Default|GetTargetLocation) (Transformation|GetActorLocation _returnvalue)))
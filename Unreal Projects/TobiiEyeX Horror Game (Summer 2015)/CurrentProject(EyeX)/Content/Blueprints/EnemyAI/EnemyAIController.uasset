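; AI controller for a horror enemy that reacts to player detection and gaze, driven by a Tick state machine.
; States park the pawn, run tutorial placement and scare events, chase via behavior tree, or follow the player until three seconds without sustained fixation trigger the chase.
; WhenDetected interpolates the pawn toward the player and plays a one-time sound, while scares set flags on MainCharacter.
; ScareEvent2 is empty and FinalEvent is a stub.
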(event EventTick
  (params (DeltaSeconds :type Float%20%28single-precision%29))
  (Variables|Default|SetDeltaSeconds DeltaSeconds)
  (switch int (Variables|Default|GetState)
    (:-1
      (Variables|Default|SetCurrentPos (Variables|Default|GetDefaultPos))
      (Transformation|SetActorLocationAndRotation (Pawn|GetControlledPawn) (Variables|Default|GetCurrentPos) (Variables|Default|GetCurrentRot)))
    (:0
      (Transformation|SetActorLocationAndRotation (Pawn|GetControlledPawn) (Variables|Default|GetCurrentPos) (Variables|Default|GetCurrentRot))
      (if (== (Variables|Default|GetEventCheck) 0)
        (if (Variables|Default|GetTutorialSetup)
          (Variables|Default|SetCurrentPos (Variables|Default|GetTutorialPos))
          (Variables|Default|SetDetection? true)
          (Variables|Default|SetTutorialSetup false)
          (elif (and (Variables|Default|GetDetection?) (Variables|Default|GetHasGaze))
            (CallFunction|WhenDetected)
            (Variables|Default|SetTimer (Utilities|Time|GetRealTimeSeconds))
            (elif (not (>= (- (Utilities|Time|GetRealTimeSeconds) (Variables|Default|GetTimer)) 3.0))
              (CallFunction|WhenDetected))))
        (elif (== (Variables|Default|GetEventCheck) 1)
          (CallFunction|ScareEvent1)
          (elif (== (Variables|Default|GetEventCheck) 2)
            (CallFunction|ScareEvent2)
            (elif (== (Variables|Default|GetEventCheck) 3)
              (CallFunction|FinalEvent))))))
    (:1
      (if (Variables|Default|GetChaseStart)
        (CallFunction|ChasePrep)
        (else
          (if (and (Variables|Default|GetDetection?) (Variables|Default|GetHasGaze))
            (bind _asmain_character (Utilities|Casting|CastToMainCharacter (Game|Player|GetPlayerPawn 0)))
            (Variables|/Game/MainCharacter.MainCharacter_C|SetChaseScare _asmain_character true))
          (Class|AIController|UseBlackboard "/Game/Blueprints/EnemyAI/EnemyBlackBoard.EnemyBlackBoard")
          (AI|RunBehaviorTree "/Game/Blueprints/EnemyAI/EnemyBehaviourTree.EnemyBehaviourTree"))))
    (:2
      (CallFunction|WhenDetected)
      (Transformation|SetActorLocationAndRotation (Pawn|GetControlledPawn) (Variables|Default|GetCurrentPos) (Variables|Default|GetCurrentRot))
      (if (not (Math|Boolean|ANDBoolean (Variables|Default|GetDetection?) (Variables|Default|GetHasGaze) (> (Variables|Default|GetFixationTime) 128.0)))
        (if (>= (- (Utilities|Time|GetRealTimeSeconds) (Variables|Default|GetTimer)) 3.0)
          (Variables|Default|SetState 1))
        (else
          (Variables|Default|SetTimer (Utilities|Time|GetRealTimeSeconds)))))))

(fn ConstructionScript)

(fn WhenDetected
  (bind _returnvalue (Pawn|GetControlledPawn))
  (bind _returnvalue_2 (Game|Player|GetPlayerPawn 0))
  (bind _returnvalue_3 (Transformation|GetActorLocation _returnvalue))
  (bind _returnvalue_4 (Transformation|GetActorLocation _returnvalue_2))
  (bind (_x _y) (Math|Vector|BreakVector _returnvalue_4))
  (Variables|Default|SetCurrentRot (Math|Interpolation|RInterpTo (Transformation|GetActorRotation (Pawn|GetControlledPawn)) (Class|KismetMathLibrary|MakeRot 0.0 (.Yaw (Class|KismetMathLibrary|BreakRot (Math|Rotator|FindLookatRotation (Transformation|GetActorLocation (Pawn|GetControlledPawn)) (Transformation|GetActorLocation (Game|Player|GetPlayerPawn 0))))) 0.0) (Variables|Default|GetDeltaSeconds) (Variables|Default|GetRotateSpeed)))
  (Variables|Default|SetCurrentPos (Math|Interpolation|VInterpTo _returnvalue_3 (Math|Vector|MakeVector _x _y (.Z (Math|Vector|BreakVector _returnvalue_3))) (Variables|Default|GetDeltaSeconds) (Variables|Default|GetFollowSpeed)))
  (Utilities|FlowControl|DoOnce false
    (:Completed
      (Audio|PlaySoundatLocation "/Game/StarterContent/Audio/Explosion02.Explosion02" (Transformation|GetActorLocation (Pawn|GetControlledPawn))))))

(fn ScareEvent1
  (Variables|Default|SetCurrentRot "0,45.000000, 0")
  (Variables|Default|SetCurrentPos "4902.440430,-10721.742188,108.714310")
  (if (Variables|Default|GetTrigger2)
    (Utilities|FlowControl|DoOnce false
      (:Completed
        (bind _asmain_character (Utilities|Casting|CastToMainCharacter (Game|Player|GetPlayerPawn 0)))
        (Variables|/Game/MainCharacter.MainCharacter_C|SetScared? _asmain_character true))))
  (if (Variables|Default|GetTrigger1)
    (Variables|Default|SetState -1)))

(fn ScareEvent2)

(fn ChasePrep
  (Transformation|SetActorLocation (Pawn|GetControlledPawn) (Variables|Default|GetChasePos) false)
  (Variables|Default|SetDetection? true))

(fn ScareInstance
  (bind _asmain_character (Utilities|Casting|CastToMainCharacter (Game|Player|GetPlayerPawn 0)))
  (Variables|/Game/MainCharacter.MainCharacter_C|SetScared? _asmain_character true))

(fn FinalEvent
  (Class|AIController|UseBlackboard))
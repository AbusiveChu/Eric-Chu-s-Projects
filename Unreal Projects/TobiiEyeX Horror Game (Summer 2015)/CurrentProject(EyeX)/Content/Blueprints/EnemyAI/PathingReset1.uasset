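; Behavior tree task for enemy AI that picks a random next pathing location from a list and writes it to the Blackboard.
; It sets the PathSet key, then reseeds its random stream while the roll matches the stored ElementCheck index, aiming to avoid repeats.
; The location write and ElementCheck update each evaluate the random roll separately, so the stored index can differ from the chosen one.
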(event EventReceiveExecute
  (params (OwnerActor :type Actor%20Object%20Reference))
  (bind _pathinglocations (Variables|Default|GetPathingLocations))
  (bind _rnjesus (Variables|Default|GetRNJesus))
  (bind _returnvalue (Utilities|Array|Length _pathinglocations))
  (bind _returnvalue_2 (- _returnvalue 1))
  (bind _returnvalue_3 (Math|Random|RandomIntegerinRangefromStream 0 _returnvalue_2 _rnjesus))
  (Class|BTFunctionLibrary|SetBlackboardValueasBool (Variables|Default|GetPathSet) true)
  (while (== (Variables|Default|GetElementCheck) _returnvalue_3)
    (Class|KismetMathLibrary|SeedRandomStream (Variables|Default|GetRNJesus)))
  (AI|BehaviorTree|SetBlackboardValueasVector (Variables|Default|GetNextPathingLocation) (Utilities|Array|Get(acopy) (Variables|Default|GetPathingLocations) _returnvalue_3))
  (Variables|Default|SetElementCheck _returnvalue_3)
  (AI|BehaviorTree|FinishExecute true))
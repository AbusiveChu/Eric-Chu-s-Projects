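; Behavior tree task that moves an EnemyAI pawn toward a blackboard target actor at a blackboard-driven speed.
; It caches the owning EnemyAIController on first execution, then sets the pawn's max walk speed from the MoveSpeed key.
; AIMoveTo follows the TargetToFollow actor, and the task finishes only on success, with no handling for a failed move or cast.
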(event EventReceiveExecute
  (params (OwnerActor :type Actor%20Object%20Reference))
  (if (!= (Variables|Default|GetAI%20CON%20Ref) 0)
    _
    (else
      (bind _asenemy_aicontroller (Utilities|Casting|CastToEnemyAIController OwnerActor))
      (Variables|Default|SetAI%20CON%20Ref _asenemy_aicontroller)))
  (bind _asenemy_ai (Utilities|Casting|CastToEnemyAI (Pawn|GetControlledPawn (Variables|Default|GetAI%20CON%20Ref))))
  (Variables|/Script/Engine.CharacterMovementComponent|SetMaxWalkSpeed (Variables|/Script/Engine.Character|GetCharacterMovement _asenemy_ai) (Class|BTFunctionLibrary|GetBlackboardValueasFloat (Variables|Default|GetMoveSpeed)))
  (AI|AIMoveTo (Pawn|GetControlledPawn (Variables|Default|GetAI%20CON%20Ref)) "0,0.000000, 0" (AI|BehaviorTree|GetBlackboardValueasActor (Variables|Default|GetTargetToFollow)) 5e+01 false
    (:OnSuccess
      (AI|BehaviorTree|FinishExecute true))))